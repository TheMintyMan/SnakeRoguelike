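; BP_ButtonAbility is an interactable ability button that shakes and pops up when picked up, extending its parent's interact logic.
; Interact starts a sound and a timeline scaled to PickUpTime, which raises the mesh from its dropping point; InteractFinished reverses it.
; Timeline curves scale Perlin noise that rotates the mesh and shakes the camera by offsetting the player pawn from its BeginPlay location.
; A timeline event triggers the pop sound or, while grabbing, plays the drop sound.
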(event EventBeginPlay
  (Variables|Default|SetOrignalCamPos (Transformation|GetActorLocation (Game|Player|GetPlayerPawn 0))))

(event EventInteract
  (params (InstigatorPawn :type SL%20Player%20Pawn%20Object%20Reference) (HitActor :type Actor%20Object%20Reference))
  (bind _buttonmesh (Variables|Default|GetButtonMesh))
  (|CallParentFunction 0 0)
  (Components|Timeline|SetPlayRate (Variables|Default|GetOneTImeline) (/ 1.0 (Variables|Default|GetPickUpTime)))
  (bind _returnvalue (Audio|SpawnSoundatLocation "/Game/Audio/Cues/SoundFX/AbilityButton/MS_AbilityButtonPop.MS_AbilityButtonPop" (Transformation|GetActorLocation) "0, 0, 0" 1.5 1.0 0.0 "/Game/Audio/Attenuation/SA_Button.SA_Button" "/Game/Audio/Concurrency/SC_Buttons.SC_Buttons" false))
  (bind (_direction _buttonshake _popup _camshake) (Timeline|OneTImeline PlayFromStart)
    (:Update
      (Variables|Default|SetTime (+ (Utilities|Time|GetWorldDeltaSeconds) (Variables|Default|GetTime)))
      (Transformation|SetActorLocation (Game|Player|GetPlayerPawn 0) (+ (Variables|Default|GetOrignalCamPos) (Math|Vector|MakeVector (.x (* (Class|KismetAnimationLibrary|MakePerlinNoiseVectorandRemap (.x (* 1e+01 (+ (+ (Utilities|Time|GetWorldDeltaSeconds) (Variables|Default|GetTime)) "0.000000,2.000000,4.000000"))) (.y (* 1e+01 (+ (+ (Utilities|Time|GetWorldDeltaSeconds) (Variables|Default|GetTime)) "0.000000,2.000000,4.000000"))) (.z (* 1e+01 (+ (+ (Utilities|Time|GetWorldDeltaSeconds) (Variables|Default|GetTime)) "0.000000,2.000000,4.000000"))) "-1.f" "1.f" "-1.f" "1.f" "-1.f" "1.f") _camshake)) (.y (* (Class|KismetAnimationLibrary|MakePerlinNoiseVectorandRemap (.x (* 1e+01 (+ (+ (Utilities|Time|GetWorldDeltaSeconds) (Variables|Default|GetTime)) "0.000000,2.000000,4.000000"))) (.y (* 1e+01 (+ (+ (Utilities|Time|GetWorldDeltaSeconds) (Variables|Default|GetTime)) "0.000000,2.000000,4.000000"))) (.z (* 1e+01 (+ (+ (Utilities|Time|GetWorldDeltaSeconds) (Variables|Default|GetTime)) "0.000000,2.000000,4.000000"))) "-1.f" "1.f" "-1.f" "1.f" "-1.f" "1.f") _camshake)) 0.0)) false false)
      (Transformation|SetWorldRotation _buttonmesh (Math|Rotator|MakeRotator (.x (* _buttonshake (Class|KismetAnimationLibrary|MakePerlinNoiseVectorandRemap (.x (* 1e+01 (+ (+ (Utilities|Time|GetWorldDeltaSeconds) (Variables|Default|GetTime)) "0.000000,2.000000,4.000000"))) (.y (* 1e+01 (+ (+ (Utilities|Time|GetWorldDeltaSeconds) (Variables|Default|GetTime)) "0.000000,2.000000,4.000000"))) (.z (* 1e+01 (+ (+ (Utilities|Time|GetWorldDeltaSeconds) (Variables|Default|GetTime)) "0.000000,2.000000,4.000000"))) "-1.f" "1.f" "-1.f" "1.f" "-1.f" "1.f"))) (.y (* _buttonshake (Class|KismetAnimationLibrary|MakePerlinNoiseVectorandRemap (.x (* 1e+01 (+ (+ (Utilities|Time|GetWorldDeltaSeconds) (Variables|Default|GetTime)) "0.000000,2.000000,4.000000"))) (.y (* 1e+01 (+ (+ (Utilities|Time|GetWorldDeltaSeconds) (Variables|Default|GetTime)) "0.000000,2.000000,4.000000"))) (.z (* 1e+01 (+ (+ (Utilities|Time|GetWorldDeltaSeconds) (Variables|Default|GetTime)) "0.000000,2.000000,4.000000"))) "-1.f" "1.f" "-1.f" "1.f" "-1.f" "1.f"))) 0.0) false false)
      (Transformation|SetWorldLocation _buttonmesh (+ (Variables|Default|GetDropppingPoint) (Math|Vector|MakeVector 0.0 0.0 _popup)) false false))
    (:NewTrack_4
      (if (Variables|Default|GetbIsGrabbing)
        (Audio|SpawnSoundatLocation "/Game/Audio/Cues/SoundFX/AbilityButton/MS_AbilityButtonDrop.MS_AbilityButtonDrop" (Transformation|GetActorLocation) "0, 0, 0" 1.0 1.0 0.0 "/Game/Audio/Attenuation/SA_Button.SA_Button" "/Game/Audio/Concurrency/SC_Buttons.SC_Buttons")
        (else
          (Class|AudioParameterControllerInterface|SetTriggerParameter _returnvalue "Pop"))))))

(event EventInteractFinished
  (params (InstigatorPawn :type SL%20Player%20Pawn%20Object%20Reference))
  (bind _buttonmesh (Variables|Default|GetButtonMesh))
  (|CallParentFunction 0)
  (bind (_direction _buttonshake _popup _camshake) (Timeline|OneTImeline Reverse)
    (:Update
      (Variables|Default|SetTime (+ (Utilities|Time|GetWorldDeltaSeconds) (Variables|Default|GetTime)))
      (Transformation|SetActorLocation (Game|Player|GetPlayerPawn 0) (+ (Variables|Default|GetOrignalCamPos) (Math|Vector|MakeVector (.x (* (Class|KismetAnimationLibrary|MakePerlinNoiseVectorandRemap (.x (* 1e+01 (+ (+ (Utilities|Time|GetWorldDeltaSeconds) (Variables|Default|GetTime)) "0.000000,2.000000,4.000000"))) (.y (* 1e+01 (+ (+ (Utilities|Time|GetWorldDeltaSeconds) (Variables|Default|GetTime)) "0.000000,2.000000,4.000000"))) (.z (* 1e+01 (+ (+ (Utilities|Time|GetWorldDeltaSeconds) (Variables|Default|GetTime)) "0.000000,2.000000,4.000000"))) "-1.f" "1.f" "-1.f" "1.f" "-1.f" "1.f") _camshake)) (.y (* (Class|KismetAnimationLibrary|MakePerlinNoiseVectorandRemap (.x (* 1e+01 (+ (+ (Utilities|Time|GetWorldDeltaSeconds) (Variables|Default|GetTime)) "0.000000,2.000000,4.000000"))) (.y (* 1e+01 (+ (+ (Utilities|Time|GetWorldDeltaSeconds) (Variables|Default|GetTime)) "0.000000,2.000000,4.000000"))) (.z (* 1e+01 (+ (+ (Utilities|Time|GetWorldDeltaSeconds) (Variables|Default|GetTime)) "0.000000,2.000000,4.000000"))) "-1.f" "1.f" "-1.f" "1.f" "-1.f" "1.f") _camshake)) 0.0)) false false)
      (Transformation|SetWorldRotation _buttonmesh (Math|Rotator|MakeRotator (.x (* _buttonshake (Class|KismetAnimationLibrary|MakePerlinNoiseVectorandRemap (.x (* 1e+01 (+ (+ (Utilities|Time|GetWorldDeltaSeconds) (Variables|Default|GetTime)) "0.000000,2.000000,4.000000"))) (.y (* 1e+01 (+ (+ (Utilities|Time|GetWorldDeltaSeconds) (Variables|Default|GetTime)) "0.000000,2.000000,4.000000"))) (.z (* 1e+01 (+ (+ (Utilities|Time|GetWorldDeltaSeconds) (Variables|Default|GetTime)) "0.000000,2.000000,4.000000"))) "-1.f" "1.f" "-1.f" "1.f" "-1.f" "1.f"))) (.y (* _buttonshake (Class|KismetAnimationLibrary|MakePerlinNoiseVectorandRemap (.x (* 1e+01 (+ (+ (Utilities|Time|GetWorldDeltaSeconds) (Variables|Default|GetTime)) "0.000000,2.000000,4.000000"))) (.y (* 1e+01 (+ (+ (Utilities|Time|GetWorldDeltaSeconds) (Variables|Default|GetTime)) "0.000000,2.000000,4.000000"))) (.z (* 1e+01 (+ (+ (Utilities|Time|GetWorldDeltaSeconds) (Variables|Default|GetTime)) "0.000000,2.000000,4.000000"))) "-1.f" "1.f" "-1.f" "1.f" "-1.f" "1.f"))) 0.0) false false)
      (Transformation|SetWorldLocation _buttonmesh (+ (Variables|Default|GetDropppingPoint) (Math|Vector|MakeVector 0.0 0.0 _popup)) false false))
    (:NewTrack_4
      (if (Variables|Default|GetbIsGrabbing)
        (Audio|SpawnSoundatLocation "/Game/Audio/Cues/SoundFX/AbilityButton/MS_AbilityButtonDrop.MS_AbilityButtonDrop" (Transformation|GetActorLocation) "0, 0, 0" 1.0 1.0 0.0 "/Game/Audio/Attenuation/SA_Button.SA_Button" "/Game/Audio/Concurrency/SC_Buttons.SC_Buttons")
        (else
          (Class|AudioParameterControllerInterface|SetTriggerParameter (stale EventInteract _returnvalue) "Pop"))))))

(fn ConstructionScript)