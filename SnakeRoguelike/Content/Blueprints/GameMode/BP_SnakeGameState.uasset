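; BP_SnakeGameState is a snake game Blueprint that shows the win/loss screen when the game ends.
; Its GameEnd event calls the parent version, then reads WinLoss from the current game state cast to SLGameStateBase.
; That value, converted to an integer, is printed and selects the active page of a WidgetSwitcher in a new WBP_WinLoss widget, which is added to the viewport.
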(event EventBeginPlay)

(event EventTick
  (params (DeltaSeconds :type Float%20%28single-precision%29)))

(event EventGameEnd
  (|CallParentFunction)
  (bind _asslgame_state_base (Utilities|Casting|CastToSLGameStateBase (Game|GetGameState)))
  (bind _returnvalue (UserInterface|CreateWidget "/Game/Blueprints/Widgets/WBP_WinLoss.WBP_WinLoss_C"))
  (Development|PrintString (Utilities|String|ToString(Integer) (Math|Conversions|ToInteger(Boolean) (Variables|/Script/SnakeRoguelike.SLGameStateBase|GetbWinLoss _asslgame_state_base))))
  (Class|WidgetSwitcher|SetActiveWidgetIndex (Variables|/Game/Blueprints/Widgets/WBP_WinLoss.WBP_WinLoss_C|GetWidgetSwitcher_39 _returnvalue) (Math|Conversions|ToInteger(Boolean) (Variables|/Script/SnakeRoguelike.SLGameStateBase|GetbWinLoss _asslgame_state_base)))
  (UserInterface|Viewport|AddtoViewport _returnvalue 0))

(fn ConstructionScript)