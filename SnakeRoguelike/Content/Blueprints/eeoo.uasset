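; Game instance (eeoo) that owns the bapbap save object in SAVE and persists it across sessions.
; Init loads it from the SlotName slot, with a branch to create and save a new one, though the preceding cast stops execution when nothing loads.
; Shutdown writes SAVE to the hardcoded "EepersSave" slot.
; Disconnected nodes that would set the save's Waawaa flag never run.
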(event EventInit
  (bind _returnvalue (SaveGame|LoadGamefromSlot (Variables|Default|GetSlot%20Name)))
  (bind _asbapbap (Utilities|Casting|CastTobapbap _returnvalue))
  (Utilities|IsValid _returnvalue
    (:Is%20Valid
      (Variables|Default|SetSAVE _asbapbap))
    (:Is%20Not%20Valid
      (bind _returnvalue_2 (SaveGame|CreateSaveGameObject "/Game/Blueprints/bapbap.bapbap_C"))
      (bind _output_get (Variables|Default|SetSAVE _returnvalue_2))
      (SaveGame|SaveGametoSlot _output_get "EepersSave"))))

(event EventShutdown
  (SaveGame|SaveGametoSlot (Variables|Default|GetSAVE) "EepersSave"))